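; LLM command component that walks its owning Character forward, backward, left or right for a requested duration.
; ExecuteCommand parses "#"-delimited direction and duration parameters, acting on the first recognised direction.
; Directions come from player controller 0's axes rather than the Character's, and Tick feeds movement input until time runs out.
; It returns an empty string, so no follow-up LLM response is triggered.
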(event EventTick
  (params (DeltaSeconds :type Float%20%28single-precision%29))
  (if (and (Variables|Default|GetbIsMoving) (Utilities|IsValid (Variables|Default|GetCharacter)))
    (Variables|Default|SetRemainingDuration (- (Variables|Default|GetRemainingDuration) DeltaSeconds))
    (Pawn|Input|AddMovementInput (Variables|Default|GetCharacter) (* 3e+02 (Variables|Default|GetDirection)) 1.0 false)
    (if (<= (Variables|Default|GetRemainingDuration) 0.0)
      (Variables|Default|SetbIsMoving false))))

(fn CanExecuteCommand
  (params (ResponseParams :type LLM%20Response%20Base%20Structure%20%28by%20ref%29))
  (bind (_message _command _target) (Utilities|Struct|BreakLLMResponseBase ResponseParams))
  (bind _returnvalue (Class|LLMCommandComponent|GetCommandStruct))
  (bind (_target_2 _name) (Utilities|Struct|BreakLLMCommandStruct _returnvalue))
  (return (and (Utilities|Enum|Equal(Enum) _target _target_2) (Utilities|Enum|Equal(Enum) _command _name))))

(fn ExecuteCommand
  (params (ResponseParams :type LLM%20Response%20Base%20Structure%20%28by%20ref%29))
  (bind _returnvalue (Game|GetPlayerController 0))
  (bind _returnvalue_2 (Transformation|GetActorForwardVector _returnvalue))
  (bind _returnvalue_3 (Transformation|GetActorRightVector _returnvalue))
  (bind _ascharacter (Utilities|Casting|CastToCharacter (Components|GetOwner)))
  (LocalVariables|SetCharacter _ascharacter)
  (bind _array_element (Utilities|Array|ForEachLoopwithBreak (.Parameters (Utilities|Struct|BreakLLMResponseBase ResponseParams)) :!label _label)
    (:LoopBody
      (bind _returnvalue_4 (Class|LLMHelperFunctionLibrary|SplitString _array_element "#" true))
      (bind (_outstring _outfloat _returnvalue_5) (Class|LLMHelperFunctionLibrary|ExtractStringandFloat _returnvalue_4))
      (if _returnvalue_5
        (switch string (Utilities|String|ToLower _outstring)
          (:forward
            (LocalVariables|SetMoveDirection _returnvalue_2))
          (:backward
            (LocalVariables|SetMoveDirection (Math|Vector|NegateVector _returnvalue_2)))
          (:left
            (LocalVariables|SetMoveDirection (Math|Vector|NegateVector _returnvalue_3)))
          (:right
            (LocalVariables|SetMoveDirection _returnvalue_3)))
        (CallFunction|StartMovement (LocalVariables|GetCharacter) (LocalVariables|GetMoveDirection) _outfloat)
        (goto _label Break)))
    (:Completed
      (return "") ; Specify an empty string if you do not want to send anything back to LLM.\nIf you want to send a request, it will provoke another response from it
    )))

(fn StartMovement
  (params (Character :type Character%20Object%20Reference) (Direction :type Vector) (Duration :type Float%20%28single-precision%29))
  (Variables|Default|SetCharacter Character)
  (Variables|Default|SetDirection Direction)
  (Variables|Default|SetRemainingDuration Duration)
  (Variables|Default|SetbIsMoving true)
  (return))